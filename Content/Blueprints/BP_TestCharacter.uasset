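; BP_TestCharacter is a test character that sets up its Gameplay Ability System attributes and abilities on OnPostBegin.
; InitializeAttribute applies max, then current gameplay effects with the same SetByCaller magnitude, seeding health and stamina from variables.
; It then self-applies stamina recovery and move speed effects via tagged SetByCaller values, and grants two attack action abilities.
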(event `self.OnPostBegin`
  (bind _abilitysystemcomponent (`self.AbilitySystemComponent`))
  (`self.InitializeAttribute` (`self.InitializeHealthValue`) "/Game/Blueprints/GameplayEffect/GE_HealthInitailize.GE_HealthInitailize_C" "/Game/Blueprints/GameplayEffect/GE_MaxHealthInitialize.GE_MaxHealthInitialize_C" (struct :`TagName` "Health.Current.Initialize") (struct :`TagName` "Health.Max.Initialize"))
  (`self.InitializeAttribute` (`self.InitializeStaminaValue`) "/Game/Blueprints/GameplayEffect/GE_StaminaInitialize.GE_StaminaInitialize_C" "/Game/Blueprints/GameplayEffect/GE_MaxStaminaInitialize.GE_MaxStaminaInitialize_C" (struct :`TagName` "Stamina.Current.Initialize") (struct :`TagName` "Stamina.Max.Initialize"))
  (bind _returnvalue (`AbilitySystemBlueprintLibrary.AssignTagSetByCallerMagnitude` (`AbilitySystemComponent.MakeOutgoingSpec` :`self` _abilitysystemcomponent :`GameplayEffectClass` "/Game/Blueprints/GameplayEffect/GE_StaminaRecovery.GE_StaminaRecovery_C") (struct :`TagName` "Stamina.Recovery") (`self.StaminaRecoveryValue`)))
  (`AbilitySystemComponent.BP_ApplyGameplayEffectSpecToTarget` _abilitysystemcomponent _returnvalue _abilitysystemcomponent)
  (bind _returnvalue_2 (`AbilitySystemBlueprintLibrary.AssignTagSetByCallerMagnitude` (`AbilitySystemComponent.MakeOutgoingSpec` :`self` _abilitysystemcomponent :`GameplayEffectClass` "/Game/Blueprints/GameplayEffect/GE_InitializeMoveSpeed.GE_InitializeMoveSpeed_C") (struct :`TagName` "MoveSpeed.Initialize") (`self.InitializeMoveSpeed`)))
  (`AbilitySystemComponent.BP_ApplyGameplayEffectSpecToTarget` _abilitysystemcomponent _returnvalue_2 _abilitysystemcomponent)
  (`ActionAbilitySystemComponent.GiveActionAbility` _abilitysystemcomponent "/Game/Ability/Action/AA_BP_Attack01.AA_BP_Attack01_C" 1 -1)
  (`ActionAbilitySystemComponent.GiveActionAbility` _abilitysystemcomponent "/Game/Blueprints/AA_BP_Attack02.AA_BP_Attack02_C" 1 -1))

(fn `InitializeAttribute`
  (params (Magnitude :type "Float (double-precision)") (CurrentInitEffect :type "GameplayEffect Class Reference") (MaxInitEffect :type "GameplayEffect Class Reference") (CurrentCallerTag :type "GameplayTag Structure") (MaxCallerTag :type "GameplayTag Structure"))
  (bind _returnvalue (`self.GetAbilitySystemComponent`))
  (bind _returnvalue_2 (`AbilitySystemBlueprintLibrary.AssignTagSetByCallerMagnitude` (`AbilitySystemComponent.MakeOutgoingSpec` :`self` _returnvalue :`GameplayEffectClass` MaxInitEffect) MaxCallerTag Magnitude))
  (`AbilitySystemComponent.BP_ApplyGameplayEffectSpecToTarget` _returnvalue _returnvalue_2 _returnvalue)
  (bind _returnvalue_3 (`AbilitySystemBlueprintLibrary.AssignTagSetByCallerMagnitude` (`AbilitySystemComponent.MakeOutgoingSpec` :`self` _returnvalue :`GameplayEffectClass` CurrentInitEffect) CurrentCallerTag Magnitude))
  (`AbilitySystemComponent.BP_ApplyGameplayEffectSpecToTarget` _returnvalue _returnvalue_3 _returnvalue))

(fn `UserConstructionScript`)